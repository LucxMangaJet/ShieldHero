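; Shield base actor that redirects projectiles through its Reflection component's custom reflection events, bound on BeginPlay.
; Reflection aims the projectile at the best enemy found in the reflected direction, keeping its speed, or falls back to a mirror bounce off the hit normal.
; After reflection, the Double modifier spawns a side-offset copy of the projectile with the same velocity and prints a debug string.
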(event `OnCustomReflection`
  (params (actor :type "Actor Object Reference") (projectileMovement :type "ProjectileMovementComponent Object Reference") (hitNormal :type "Vector Structure"))
  (bind _returnvalue (`self.K2_GetActorLocation` actor))
  (bind _returnvalue_2 (`ReflectionComponent.FindBestEnemyInDirectionAfterReflection` (`self.Reflection`) _returnvalue hitNormal (`MovementComponent.Velocity` projectileMovement) 50000.0))
  (`/Engine/EditorBlueprintResources/StandardMacros.IsValid` _returnvalue_2
    (:`Is Valid`
      (bind _returnvalue_3 (* (`KismetMathLibrary.Normal` (- (`self.K2_GetActorLocation` _returnvalue_2) _returnvalue)) (`KismetMathLibrary.VSize` (`MovementComponent.Velocity` projectileMovement))))
      (set `MovementComponent.Velocity` _returnvalue_3 projectileMovement)
      (`self.K2_SetActorRotation` actor (`KismetMathLibrary.MakeRotFromX` _returnvalue_3) false))
    (:`Is Not Valid`
      (bind _output_get (set `MovementComponent.Velocity` (`KismetMathLibrary.GetReflectionVector` (`MovementComponent.Velocity` projectileMovement) hitNormal) projectileMovement))
      (`self.K2_SetActorRotation` actor (`KismetMathLibrary.MakeRotFromX` _output_get) false))))

(event `self.ReceiveBeginPlay`
  (bind _reflection (`self.Reflection`))
  (add `ReflectionComponent.OnCustomReflection` _reflection (delegate `OnCustomReflection`))
  (add `ReflectionComponent.OnPostCustomReflection` _reflection (delegate `OnPostCustomReflection_Event_0`)))

(event `OnPostCustomReflection_Event_0`
  (params (actor :type "Actor Object Reference") (projectileMovement :type "ProjectileMovementComponent Object Reference"))
  (bind (_returnvalue_location _returnvalue_rotation _returnvalue_scale) (`KismetMathLibrary.BreakTransform` (`self.GetTransform` actor)))
  (switch `ShieldReflectionModifier` (`ReflectionComponent._reflectionModifier` (`self.Reflection`))
    (:`Double`
      (bind _returnvalue (`|SpawnActorFromClass` (`GameplayStatics.GetObjectClass` actor) (`KismetMathLibrary.MakeTransform` (+ _returnvalue_location (* (`KismetMathLibrary.GetRightVector` _returnvalue_rotation) 30.0)) _returnvalue_rotation _returnvalue_scale) "AlwaysSpawn" "OverrideRootScale" null null))
      (set `MovementComponent.Velocity` (`MovementComponent.Velocity` projectileMovement) (`self.GetComponentByClass` _returnvalue "/Script/Engine.ProjectileMovementComponent"))
      (`KismetSystemLibrary.PrintString` "Hello"))))

(fn `UserConstructionScript`)