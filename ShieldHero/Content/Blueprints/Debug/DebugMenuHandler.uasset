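; Debug actor that spawns the debug master and main menu widgets and routes input to them.
; On BeginPlay it enables input for player 0, creates both widgets and adds them to the viewport.
; The ToggleDebug input toggles the debug menu, and MainMenuDebug shows the main menu.
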(event `self.ReceiveBeginPlay`
  (`self.EnableInput` (`GameplayStatics.GetPlayerController` 0))
  (`|ExecutionSequence`
    (:`then_0`
      (bind _returnvalue (`|CreateWidget` "/Game/UI/Debug/WB_DebugMaster.WB_DebugMaster_C" (`GameplayStatics.GetPlayerController` 0)))
      (bind _output_get (set `self.DebugMenu` _returnvalue))
      (`UserWidget.AddToViewport` _output_get 0))
    (:`then_1`
      (bind _returnvalue_2 (`|CreateWidget` "/Game/UI/Widgets/WB_MainMenu.WB_MainMenu_C" (`GameplayStatics.GetPlayerController` 0)))
      (bind _output_get_2 (set `self.MainMenu` _returnvalue_2))
      (`UserWidget.AddToViewport` _output_get_2 0))))

(event `InputAction|ToggleDebug` :consume false :overrideparent false
  (params (Key :type "Key Structure"))
  (:`Pressed`
    (`/Game/UI/Debug/WB_DebugMaster.ToggleDebug` (`self.DebugMenu`))))

(event `InputAction|MainMenuDebug`
  (params (Key :type "Key Structure"))
  (:`Pressed`
    (`/Game/UI/Widgets/WB_MainMenu.Show Menu` (`self.MainMenu`))))

(fn `UserConstructionScript`)