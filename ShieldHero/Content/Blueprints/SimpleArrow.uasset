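; SimpleArrow is a projectile arrow that reacts to surfaces it overlaps by bouncing or sticking, dealing damage on some hits.
; On overlap, gated by a HitStamp time check, a short forward trace reads the hit actor's ReflectionComponent type.
; That type selects mirrored reflection, normal-directed bounce, reflect with damage, or attach with damage; surfaces without the component reflect.
; Bounces change the arrow's material and turn its emitter green.
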(event `self.ReceiveActorBeginOverlap`
  (params (OtherActor :type "Actor Object Reference"))
  (bind _returnvalue (`self.K2_GetActorLocation`))
  (bind _projectilemovement (`self.ProjectileMovement`))
  (bind _projectilemovement_2 (`self.ProjectileMovement`))
  (if (> (- (`GameplayStatics.GetTimeSeconds`) (`self.hitStamp`)) 0.1)
    (bind (_outhit _returnvalue_2) (`KismetSystemLibrary.LineTraceSingle` _returnvalue (+ _returnvalue (* (`self.GetActorForwardVector`) 50.0)) "TraceTypeQuery1" true))
    (if _returnvalue_2
      (bind _returnvalue_3 (`self.GetComponentByClass` (`.HitActor` (`GameplayStatics.BreakHitResult` _outhit)) "/Script/ShieldHero.ReflectionComponent"))
      (`/Engine/EditorBlueprintResources/StandardMacros.IsValid` _returnvalue_3
        (:`Is Valid`
          (switch `ReflectionType` (`ReflectionComponent._reflectionType` _returnvalue_3)
            (:`Reflect`
              (bind _output_get (set `MovementComponent.Velocity` (`KismetMathLibrary.GetReflectionVector` (`MovementComponent.Velocity` _projectilemovement) (`.Normal` (`GameplayStatics.BreakHitResult` _outhit))) _projectilemovement :!label _label))
              (`self.K2_SetActorRotation` (`KismetMathLibrary.MakeRotFromX` _output_get))
              (`PrimitiveComponent.SetMaterial` (`self.StaticMesh`) 0 "/Engine/MapTemplates/Materials/BasicAsset03.BasicAsset03" :!label _label_2)
              (`FXSystemComponent.SetColorParameter` (`self.GenericEmitter`) "Color" (struct :`G` 1.0 :`A` 1.0)))
            (:`StopAndDamage`
              (`PrimitiveComponent.SetCollisionEnabled` (`self.Box`) "NoCollision")
              (`MovementComponent.StopMovementImmediately` (`self.ProjectileMovement`))
              (`self.K2_AttachToActor` (`.HitActor` (`GameplayStatics.BreakHitResult` _outhit)) "None" "KeepWorld" "KeepWorld" "KeepWorld")
              (`/Game/Blueprints/ShieldHeroFunctionLibrary.Try Deal Damage` (`.HitActor` (`GameplayStatics.BreakHitResult` _outhit)) (`self.Damage`))
              (`ActorComponent.K2_DestroyComponent` (`self.GenericEmitter`)))
            (:`ReflectAndDamage`
              (`/Game/Blueprints/ShieldHeroFunctionLibrary.Try Deal Damage` (`.HitActor` (`GameplayStatics.BreakHitResult` _outhit)) (`self.Damage`))
              (goto _label))
            (:`ReflectDirected`
              (bind _output_get_2 (set `MovementComponent.Velocity` (* (`.Normal` (`GameplayStatics.BreakHitResult` _outhit)) (`KismetMathLibrary.VSize` (`MovementComponent.Velocity` _projectilemovement_2))) _projectilemovement_2))
              (`self.K2_SetActorRotation` (`KismetMathLibrary.MakeRotFromX` _output_get_2))
              (goto _label_2))))
        (:`Is Not Valid`
          (goto _label))))))

(fn `UserConstructionScript`)