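; HealthBar_BP is a widget component that displays a health bar for the actor that owns it.
; On BeginPlay it switches to absolute rotation and orients itself once from the player camera's up vector with a 180-degree roll, so it ignores the owner's rotation.
; It then finds the owner's HealthComponent and, if valid, passes it to the WB_GenericHealthBar widget's Setup.
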(event `self.ReceiveBeginPlay`
  (bind _returnvalue (`Actor.GetComponentByClass` (`self.GetOwner`) "/Script/ShieldHero.HealthComponent"))
  (set `self.bAbsoluteRotation` true)
  (`self.K2_SetWorldRotation` (`KismetMathLibrary.ComposeRotators` (`KismetMathLibrary.Conv_VectorToRotator` (`KismetMathLibrary.GetUpVector` (`PlayerCameraManager.GetCameraRotation` (`GameplayStatics.GetPlayerCameraManager` 0)))) (struct :`Yaw` 180.0)))
  (`/Engine/EditorBlueprintResources/StandardMacros.IsValid` _returnvalue
    (:`Is Valid`
      (bind _aswb_generic_health_bar (cast `/Game/UI/Widgets/WB_GenericHealthBar` (`self.GetWidget`)))
      (`/Game/UI/Widgets/WB_GenericHealthBar.Setup` _aswb_generic_health_bar _returnvalue))))