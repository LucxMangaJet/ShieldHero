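; Level door that opens when the game is won and closes after the hero passes through its trigger.
; On BeginPlay it binds to the KillAllGameMode game-won event, which plays a timeline sliding the inner door piece along Z.
; Once fully open, a ShieldHeroCharacter ending overlap with the trigger plays a second timeline in reverse to slide it back and clear the open flag.
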(event `self.ReceiveBeginPlay`
  (bind _askill_all_game_mode (cast `KillAllGameMode` (`GameplayStatics.GetGameMode`)))
  (add `KillAllGameMode.OnGameWon` _askill_all_game_mode (delegate `OnGameWon`)))

(event `OnGameWon`
  (bind (_direction _slideamount) (`Timeline|DoorAnimation` :!via `PlayFromStart`)
    (:`Update`
      (`SceneComponent.K2_SetRelativeLocation` (`self.InnerDoorPiece`) (`KismetMathLibrary.MakeVector` 0.0 0.0 (* _slideamount 100.0)) false false))
    (:`Finished`
      (set `self.IsOpen` true))))

(event `self.DoorTrigger.OnComponentEndOverlap`
  (params (OverlappedComponent :type "PrimitiveComponent Object Reference") (OtherActor :type "Actor Object Reference") (OtherComp :type "PrimitiveComponent Object Reference") (OtherBodyIndex :type Integer))
  (if (`self.IsOpen`)
    (cast `ShieldHeroCharacter` OtherActor)
    (bind (_direction _slideamount) (`Timeline|DoorReturn` :!via `ReverseFromEnd`)
      (:`Update`
        (`SceneComponent.K2_SetRelativeLocation` (`self.InnerDoorPiece`) (`KismetMathLibrary.MakeVector` 0.0 0.0 (* _slideamount 100.0)) false false))
      (:`Finished`
        (set `self.IsOpen` false)))))

(fn `UserConstructionScript`)