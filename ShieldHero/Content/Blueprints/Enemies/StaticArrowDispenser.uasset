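; An enemy dispenser actor that repeatedly spawns projectiles or other actors of a configurable Source class.
; A looping timer started on BeginPlay fires every Delay seconds and spawns at the Arrow component's world transform, with no aiming logic.
; A Health component's OnDeath event destroys the dispenser.
; The player pawn is cached on BeginPlay but not used in these graphs.
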(event `self.ReceiveBeginPlay`
  (`KismetSystemLibrary.K2_SetTimerDelegate` (delegate `TimerEvent`) (`self.Delay`) true)
  (add `HealthComponent.OnDeath` (`self.Health`) (delegate `OnDeath_Event_0`))
  (set `self.Player` (`GameplayStatics.GetPlayerPawn` 0)))

(event `TimerEvent`
  (`|SpawnActorFromClass` (`self.Source`) (`SceneComponent.K2_GetComponentToWorld` (`self.Arrow`)) "Undefined" "OverrideRootScale" null null))

(event `OnDeath_Event_0`
  (`self.K2_DestroyActor`))

(fn `UserConstructionScript`)