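; An enemy turret that keeps turning to face the player and periodically spawns projectiles or other actors of a configurable class.
; A looping timer spawns the Source class at the Arrow component's transform, at an interval set by Delay.
; Tick rotates the whole actor toward the first player pawn, cached on BeginPlay, using only X and Y positions.
; The Health component's death event destroys the dispenser.
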(event `self.ReceiveBeginPlay`
  (`KismetSystemLibrary.K2_SetTimerDelegate` (delegate `TimerEvent`) (`self.Delay`) true)
  (add `HealthComponent.OnDeath` (`self.Health`) (delegate `OnDeath_Event_0`))
  (set `self.Player` (`GameplayStatics.GetPlayerPawn` 0)))

(event `TimerEvent`
  (`|SpawnActorFromClass` (`self.Source`) (`SceneComponent.K2_GetComponentToWorld` (`self.Arrow`)) "Undefined" "OverrideRootScale" null null))

(event `OnDeath_Event_0`
  (`self.K2_DestroyActor`))

(event `self.ReceiveTick`
  (params (DeltaSeconds :type "Float (single-precision)"))
  (bind (_returnvalue_x _returnvalue_y) (`KismetMathLibrary.BreakVector` (`self.K2_GetActorLocation`)))
  (bind (_returnvalue_x_2 _returnvalue_y_2) (`KismetMathLibrary.BreakVector` (`self.K2_GetActorLocation` (`self.Player`))))
  (`self.K2_SetActorRotation` (`KismetMathLibrary.FindLookAtRotation` (`KismetMathLibrary.MakeVector` _returnvalue_x _returnvalue_y) (`KismetMathLibrary.MakeVector` _returnvalue_x_2 _returnvalue_y_2))))

(fn `UserConstructionScript`)