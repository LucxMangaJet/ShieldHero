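; BP_ShieldHero is a hero Blueprint with a health component and a prototype scalable shield.
; On BeginPlay it binds to the health component's death event, which reloads the current level by name.
; Two exploratory custom events grow the Shield's Y scale by one per call or reset it to uniform scale; neither is called within this graph.
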(event `self.ReceiveBeginPlay`
  (add `HealthComponent.OnDeath` (`self._healthComponent`) (delegate `OnDeath`)))

(event `OnDeath`
  (bind _returnvalue (`GameplayStatics.GetCurrentLevelName` true))
  (`GameplayStatics.OpenLevel` (`KismetStringLibrary.Conv_StringToName` _returnvalue)))

(event `ScaleShield Y`
  (bind __shield (`self._shield`))
  (bind (_relativescale3d_x _relativescale3d_y _relativescale3d_z) (`KismetMathLibrary.BreakVector` (`SceneComponent.RelativeScale3D` __shield)))
  ;[1 1 1] Shield Proto exploration
  (`SceneComponent.SetRelativeScale3D` __shield (`KismetMathLibrary.MakeVector` _relativescale3d_x (+ _relativescale3d_y 1.0) _relativescale3d_z)))

(event `Reset Shield`
  ;[1 1 1] Shield Proto exploration
  (`SceneComponent.SetRelativeScale3D` (`self._shield`) (1.0 1.0 1.0)))

(fn `UserConstructionScript`)