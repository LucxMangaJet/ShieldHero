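; Camera actor that follows the first player's pawn along X and Z while holding Y constant.
; At BeginPlay it caches the pawn, builds an offset from its own world X and its relative Y and Z to the pawn, then becomes the player controller's view target.
; Each Tick it moves to the pawn's X and Z plus that offset, without smoothing or sweep.
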(event `self.ReceiveBeginPlay`
  (bind _returnvalue (`self.K2_GetActorLocation`))
  (bind _output_get (set `self.Target` (`GameplayStatics.GetPlayerPawn` 0)))
  (bind (_returnvalue_x _returnvalue_y _returnvalue_z) (`KismetMathLibrary.BreakVector` (- _returnvalue (`self.K2_GetActorLocation` _output_get))))
  (set `self.Offset` (`KismetMathLibrary.MakeVector` (.x _returnvalue) _returnvalue_y _returnvalue_z))
  (`PlayerController.SetViewTargetWithBlend` (`GameplayStatics.GetPlayerController` 0) self 0.0 "VTBlend_Linear" 0.0 false))

(event `self.ReceiveTick`
  (params (DeltaSeconds :type "Float (single-precision)"))
  (bind (_returnvalue_x _returnvalue_y _returnvalue_z) (`KismetMathLibrary.BreakVector` (`self.K2_GetActorLocation` (`self.Target`))))
  (`self.K2_SetActorLocation` (+ (`KismetMathLibrary.MakeVector` _returnvalue_x 0.0 _returnvalue_z) (`self.Offset`))))

(fn `UserConstructionScript`)