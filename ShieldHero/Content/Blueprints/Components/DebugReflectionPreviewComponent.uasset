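; Scene component that previews how a ray bounces off surfaces by drawing debug lines from its world location along its forward vector.
; DebugVisualize starts a recursive trace on the Visibility channel using complex collision.
; Each hit draws a segment and recurses along the reflected direction until DrawSteps runs out, while a miss draws one long final segment and stops.
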(event `DebugVisualize`
  (`self.DebugVisualizeInternal` (`self.K2_GetComponentLocation`) (`self.GetForwardVector`) (`self.DrawSteps`) (`self.DrawDuration`)))

(fn `DebugVisualizeInternal`
  (params (InPosition :type "Vector Structure") (InForward :type "Vector Structure") (MaxSteps :type Integer) (Duration :type "Float (double-precision)"))
  (bind _returnvalue (+ InPosition (* InForward 100000)))
  (if (> MaxSteps 0)
    (bind (_outhit _returnvalue_2) (`KismetSystemLibrary.LineTraceSingle` InPosition _returnvalue "TraceTypeQuery1" true))
    (if _returnvalue_2
      (bind (_bblockinghit _binitialoverlap _time _distance _location _impactpoint _normal) (`GameplayStatics.BreakHitResult` _outhit))
      (`KismetSystemLibrary.DrawDebugLine` (`local.InPosition`) _impactpoint (struct :`R` 0.023153 :`B` 1.0 :`A` 1.0) (`local.Duration`) 5.0)
      (`self.DebugVisualizeInternal` _impactpoint (`KismetMathLibrary.GetReflectionVector` (`local.InForward`) _normal) (- (`local.MaxSteps`) 1) (`local.Duration`))
      (else
        (`KismetSystemLibrary.DrawDebugLine` (`local.InPosition`) _returnvalue (struct :`R` 0.023153 :`B` 1.0 :`A` 1.0) (`local.Duration`) 5.0)))))