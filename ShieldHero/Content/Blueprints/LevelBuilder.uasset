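; LevelBuilder is a Blueprint that procedurally fills a rectangular floor area with randomly chosen static meshes.
; BuildLvl runs from both the Construction Script and BeginPlay, rebuilding a grid of transforms from the X/Y extents and step size, each with random quarter-turn yaw.
; It then adds a mesh component per transform, applying SceneTexture_MAT and a random mesh from NewMesh.
; BeginPlay does not remove existing components before adding its own.
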(event `self.ReceiveBeginPlay`
  (`self.BuildLvl`))

(fn `BuildLvl`
  (`KismetArrayLibrary.Array_Clear` (`self.Locations`))
  (set `self.Counter_X` 0)
  (set `self.Helper Vector` (0.0 0.0 0.0))
  (for _ (range 1 (+ (/ (`self.X_MaxPosition`) (`self.StepSize`)) 1))
    (for _ (range 1 (+ (/ (`self.Y_MaxPosition`) (`self.StepSize`)) 1))
      (bind _output_get (set `self.Helper Vector` (`KismetMathLibrary.MakeVector` (`KismetMathLibrary.Conv_IntToDouble` (`self.Counter_X`)) (`KismetMathLibrary.Conv_IntToDouble` (`self.Counter_Y`)))))
      (`KismetArrayLibrary.Array_Add` (`self.Locations`) (`KismetMathLibrary.MakeTransform` _output_get (`KismetMathLibrary.MakeRotator` 0.0 0.0 (`KismetMathLibrary.Conv_IntToDouble` (* (`KismetMathLibrary.RandomIntegerInRange` 0 3) 90)))))
      (set `self.Counter_Y` (+ (`self.StepSize`) (`self.Counter_Y`))))
    (set `self.Counter_Y` 0)
    (set `self.Counter_X` (+ (`self.StepSize`) (`self.Counter_X`))))
  (for _array_element (`self.Locations`)
    (bind _returnvalue (`AddComponent|NODE_AddStaticMeshComponent-0` :`RelativeTransform` _array_element))
    (`PrimitiveComponent.SetMaterial` _returnvalue 0 "/Game/Environment/BaseGeo/SceneTexture_MAT.SceneTexture_MAT")
    (`StaticMeshComponent.SetStaticMesh` _returnvalue (`KismetArrayLibrary.Array_Random` (`self.New Mesh`)))))

(fn `UserConstructionScript`
  (`self.BuildLvl`))